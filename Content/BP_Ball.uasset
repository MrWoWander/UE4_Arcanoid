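; BP_Ball is a ball actor that travels in a straight line and bounces off whatever it hits.
; It takes its initial direction from the actor's forward vector, then moves each Tick by Speed with a swept world offset, without physics simulation.
; On a blocking hit it reflects the direction about the surface normal and rotates to face it.
; A 5% speed increase node exists but is unconnected, so Speed stays constant.
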(event `self.ReceiveBeginPlay`
  (set `self.Direction` (`self.GetActorForwardVector`)))

(event `self.ReceiveTick`
  (params (DeltaSeconds :type "Float (single-precision)"))
  (bind _sweephitresult (`self.K2_AddActorWorldOffset` (* (`self.Direction`) (* (`self.Speed`) DeltaSeconds)) true))
  (bind (_bblockinghit _binitialoverlap _time _distance _location _impactpoint _normal) (`GameplayStatics.BreakHitResult` _sweephitresult))
  (if _bblockinghit
    (bind _output_get (set `self.Direction` (`KismetMathLibrary.GetReflectionVector` (`self.Direction`) _normal)))
    (`self.K2_SetActorRotation` (`KismetMathLibrary.Conv_VectorToRotator` _output_get))))

(fn `UserConstructionScript`)